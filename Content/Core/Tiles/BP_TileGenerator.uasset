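; BP_TileGenerator spawns a hex or square grid of BP_Tile actors on BeginPlay, selected by the Hex flag.
; Hex rows alternate through a FlipFlop to offset every other row by half a tile, while both layouts set the tile shape to Hex.
; Each tile receives coordinates and a running index into the Tiles array, presized in the construction script.
; GetCellAtCoordinate reads that flat array using GridSize.Value1 as stride, although generated rows are Value2 long.
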(event `self.ReceiveBeginPlay`
  (bind (_gridsize_value1 _gridsize_value2) (break `/Game/Core/Int2D` (`self.GridSize`)))
  (bind _tiles (`self.Tiles`))
  (bind _currentindex (`self.CurrentIndex`))
  (bind (_gridsize_value1_2 _gridsize_value2_2) (break `/Game/Core/Int2D` (`self.GridSize`)))
  (bind _currentindex_2 (`self.CurrentIndex`))
  (bind _currentindex_3 (`self.CurrentIndex`))
  (bind _hex_ (`self.Hex?`))
  (bind _returnvalue (- _gridsize_value2_2 1))
  (if (`self.Hex?`)
    ;[0.4769 1 0.6925] Create Hex Grid
    (for _index (range _gridsize_value1_2)
      (`/Engine/EditorBlueprintResources/StandardMacros.FlipFlop`
        (:`A`
          (for _index_2 (range (+ _returnvalue 1))
            (bind _returnvalue_2 (* _index 75.0))
            (bind _returnvalue_3 (`|SpawnActorFromClass` "/Game/Core/Tiles/BP_Tile.BP_Tile_C" (`KismetMathLibrary.MakeTransform` (`KismetMathLibrary.MakeVector` (* _index_2 86.5) _returnvalue_2)) "Undefined" "OverrideRootScale" null null))
            (`/Game/Core/Tiles/BP_Tile.SetShape` _returnvalue_3 _hex_)
            (`/Game/Core/Tiles/BP_Tile.SetCoordinates` _returnvalue_3 (make `/Game/Core/Int2D` _index_2 _index) _currentindex)
            (`KismetArrayLibrary.Array_Set` _tiles _currentindex_2 _returnvalue_3)
            (`/Engine/EditorBlueprintResources/StandardMacros.IncrementInt` (`self.CurrentIndex`) :!label _label)))
        (:`B`
          (for _index_3 (range (+ _returnvalue 1))
            (bind _returnvalue_4 (`|SpawnActorFromClass` "/Game/Core/Tiles/BP_Tile.BP_Tile_C" (`KismetMathLibrary.MakeTransform` (`KismetMathLibrary.MakeVector` (+ (* _index_3 86.5) 43.25) _returnvalue_2)) "Undefined" "OverrideRootScale" null null))
            (`/Game/Core/Tiles/BP_Tile.SetShape` _returnvalue_4 _hex_)
            (`/Game/Core/Tiles/BP_Tile.SetCoordinates` _returnvalue_4 (make `/Game/Core/Int2D` _index_3 _index) _currentindex)
            (`KismetArrayLibrary.Array_Set` _tiles _currentindex_2 _returnvalue_4)
            (goto _label)))))
    (else
      ;[1 0.7952 0.6084] Create Square Grid
      (for _index_4 (range _gridsize_value1)
        (for _index_5 (range _gridsize_value2)
          (bind _returnvalue_5 (`|SpawnActorFromClass` "/Game/Core/Tiles/BP_Tile.BP_Tile_C" (`KismetMathLibrary.MakeTransform` (`KismetMathLibrary.MakeVector` (* _index_5 100.0) (* _index_4 100.0))) "Undefined" "OverrideRootScale" null null))
          (`/Game/Core/Tiles/BP_Tile.SetShape` _returnvalue_5 (`self.Hex?`))
          (`/Game/Core/Tiles/BP_Tile.SetCoordinates` _returnvalue_5 (make `/Game/Core/Int2D` _index_5 _index_4) _currentindex_3)
          (`KismetArrayLibrary.Array_Set` (`self.Tiles`) _currentindex_3 _returnvalue_5)
          (`/Engine/EditorBlueprintResources/StandardMacros.IncrementInt` (`self.CurrentIndex`)))))))

(fn `GetCellAtCoordinate`
  (params (Coordinate :type "/Game/Core/Int2D Structure"))
  (returns (TileRef :type "/Game/Core/Tiles/BP_Tile Object Reference"))
  (bind _gridsize_value1 (break `/Game/Core/Int2D` (`self.GridSize`)))
  (return (`|GetArrayItem` (`self.Tiles`) (+ Coordinate_Value1_2_0D60888443DB7109C5060C8AE787FDE6 (* Coordinate_Value2_4_1B0FBEA646C06A4A8B3183871708624D _gridsize_value1)))))

(fn `UserConstructionScript`
  (bind (_gridsize_value1 _gridsize_value2) (break `/Game/Core/Int2D` (`self.GridSize`)))
  (`KismetArrayLibrary.Array_Resize` (`self.Tiles`) (* _gridsize_value1 _gridsize_value2)))