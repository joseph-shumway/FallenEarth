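; BP_Tile is a map tile that shows either a square or hexagon mesh and takes on a random biome look.
; The construction script calls SetShape with the Hex flag to toggle mesh visibility, then assigns one of nine biome materials to both meshes.
; The random roll is evaluated separately for the stored Biome and the material switch, so the two can differ.
; The event graph holds only disabled stubs.
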(fn `SetShape`
  (params (`Hexagon?` :type Boolean))
  (if `Hexagon?`
    (`SceneComponent.SetVisibility` (`self.Hexagon`) true false)
    (`SceneComponent.SetVisibility` (`self.Square`) false false)
    (else
      (`SceneComponent.SetVisibility` (`self.Hexagon`) false false)
      (`SceneComponent.SetVisibility` (`self.Square`) true false)))
  (return))

(fn `UserConstructionScript`
  (bind _square (`self.Square`))
  (bind _returnvalue (cast `/Game/Core/Tiles/Biome_Enum` (`KismetMathLibrary.Conv_IntToByte` (`KismetMathLibrary.RandomIntegerInRange` 0 8))))
  (`self.SetShape` (`self.Hex?`))
  (set `self.Biome` _returnvalue)
  (switch `/Game/Core/Tiles/Biome_Enum` _returnvalue
    (:`NewEnumerator0`
      (`PrimitiveComponent.SetMaterial` _square 0 "/Game/Core/Tiles/MI_Biome_Desert.MI_Biome_Desert")
      (`PrimitiveComponent.SetMaterial` (`self.Hexagon`) 0 "/Game/Core/Tiles/MI_Biome_Desert.MI_Biome_Desert"))
    (:`NewEnumerator1`
      (`PrimitiveComponent.SetMaterial` _square 0 "/Game/Core/Tiles/MI_Biome_Grasslands.MI_Biome_Grasslands")
      (`PrimitiveComponent.SetMaterial` (`self.Hexagon`) 0 "/Game/Core/Tiles/MI_Biome_Grasslands.MI_Biome_Grasslands"))
    (:`NewEnumerator3`
      (`PrimitiveComponent.SetMaterial` _square 0 "/Game/Core/Tiles/MI_Biome_Ocean.MI_Biome_Ocean")
      (`PrimitiveComponent.SetMaterial` (`self.Hexagon`) 0 "/Game/Core/Tiles/MI_Biome_Ocean.MI_Biome_Ocean"))
    (:`NewEnumerator7`
      (`PrimitiveComponent.SetMaterial` _square 0 "/Game/Core/Tiles/MI_Biome_TropicalForest.MI_Biome_TropicalForest")
      (`PrimitiveComponent.SetMaterial` (`self.Hexagon`) 0 "/Game/Core/Tiles/MI_Biome_TropicalForest.MI_Biome_TropicalForest"))
    (:`NewEnumerator8`
      (`PrimitiveComponent.SetMaterial` _square 0 "/Game/Core/Tiles/MI_Biome_TempForest.MI_Biome_TempForest")
      (`PrimitiveComponent.SetMaterial` (`self.Hexagon`) 0 "/Game/Core/Tiles/MI_Biome_TempForest.MI_Biome_TempForest"))
    (:`NewEnumerator9`
      (`PrimitiveComponent.SetMaterial` _square 0 "/Game/Core/Tiles/MI_Biome_Taiga.MI_Biome_Taiga")
      (`PrimitiveComponent.SetMaterial` (`self.Hexagon`) 0 "/Game/Core/Tiles/MI_Biome_Taiga.MI_Biome_Taiga"))
    (:`NewEnumerator10`
      (`PrimitiveComponent.SetMaterial` _square 0 "/Game/Core/Tiles/MI_Biome_Tundra.MI_Biome_Tundra")
      (`PrimitiveComponent.SetMaterial` (`self.Hexagon`) 0 "/Game/Core/Tiles/MI_Biome_Tundra.MI_Biome_Tundra"))
    (:`NewEnumerator11`
      (`PrimitiveComponent.SetMaterial` _square 0 "/Game/Core/Tiles/MI_Biome_Volcanic.MI_Biome_Volcanic")
      (`PrimitiveComponent.SetMaterial` (`self.Hexagon`) 0 "/Game/Core/Tiles/MI_Biome_Volcanic.MI_Biome_Volcanic"))
    (:`NewEnumerator12`
      (`PrimitiveComponent.SetMaterial` _square 0 "/Game/Core/Tiles/MI_Biome_Marsh.MI_Biome_Marsh")
      (`PrimitiveComponent.SetMaterial` (`self.Hexagon`) 0 "/Game/Core/Tiles/MI_Biome_Marsh.MI_Biome_Marsh"))))