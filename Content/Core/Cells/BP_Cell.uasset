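; BP_Cell is a map grid tile that shows a hexagon or square mesh with one of nine biome materials.
; Construction sets the shape and a random biome, rolling separately for the stored biome and the material, so they can differ.
; It stores hex coordinates and grid index, displaying them with a derived cube Y as text.
; SetNeighbor links two cells both ways by indexing neighbor arrays with direction and its opposite.
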(fn `FromOffsetCoordinates`
  (params (Coordinates :type "/Game/Core/RegCoordinates Structure"))
  (returns (HexCoordinates :type "/Game/Core/HexCoordinates Structure"))
  (return (make `/Game/Core/HexCoordinates` (- Coordinates_X_5_0D60888443DB7109C5060C8AE787FDE6 (/ Coordinates_Z_7_1B0FBEA646C06A4A8B3183871708624D 2)) Coordinates_Z_7_1B0FBEA646C06A4A8B3183871708624D)))

(fn `getHexYCoord`
  (params (X :type Integer) (Z :type Integer))
  (returns (Y :type Integer))
  (return (- (* X -1) Z)))

(fn `getNeighbor`
  (params (Direction :type "/Game/Core/Cells/HexDirection_Enum Enum" :default "NewEnumerator0"))
  (returns (Neighbor :type "/Game/Core/Cells/BP_Cell Object Reference"))
  (return (`|GetArrayItem` (`self.Neighbors`) (`KismetMathLibrary.Conv_ByteToInt` Direction))))

(fn `getOppositeDirection`
  (params (Direction :type "/Game/Core/Cells/HexDirection_Enum Enum" :default "NewEnumerator0"))
  (returns (Opposite :type "/Game/Core/Cells/HexDirection_Enum Enum"))
  (bind _returnvalue (`KismetMathLibrary.Conv_ByteToInt` Direction))
  (if (< _returnvalue 3)
    (return (cast `/Game/Core/Cells/HexDirection_Enum` (`KismetMathLibrary.Conv_IntToByte` (+ _returnvalue 3))))
    (else
      (return (cast `/Game/Core/Cells/HexDirection_Enum` (`KismetMathLibrary.Conv_IntToByte` (- _returnvalue 3)))))))

(fn `setBiome`
  (params (`Random?` :type Boolean) (Biome :type "/Game/Core/Cells/Biome_Enum Enum" :default "NewEnumerator0"))
  (bind _square (`self.Square`))
  (bind _square_2 (`self.Square`))
  (bind _returnvalue (cast `/Game/Core/Cells/Biome_Enum` (`KismetMathLibrary.Conv_IntToByte` (`KismetMathLibrary.RandomIntegerInRange` 0 8))))
  (if `Random?`
    (set `self.Biome` _returnvalue)
    (switch `/Game/Core/Cells/Biome_Enum` _returnvalue
      (:`NewEnumerator0`
        (`PrimitiveComponent.SetMaterial` _square_2 0 "/Game/Core/Cells/MI_Biome_Desert.MI_Biome_Desert")
        (`PrimitiveComponent.SetMaterial` (`self.Hexagon`) 0 "/Game/Core/Cells/MI_Biome_Desert.MI_Biome_Desert"))
      (:`NewEnumerator1`
        (`PrimitiveComponent.SetMaterial` _square_2 0 "/Game/Core/Cells/MI_Biome_Grasslands.MI_Biome_Grasslands")
        (`PrimitiveComponent.SetMaterial` (`self.Hexagon`) 0 "/Game/Core/Cells/MI_Biome_Grasslands.MI_Biome_Grasslands"))
      (:`NewEnumerator12`
        (`PrimitiveComponent.SetMaterial` _square_2 0 "/Game/Core/Cells/MI_Biome_Marsh.MI_Biome_Marsh")
        (`PrimitiveComponent.SetMaterial` (`self.Hexagon`) 0 "/Game/Core/Cells/MI_Biome_Marsh.MI_Biome_Marsh"))
      (:`NewEnumerator3`
        (`PrimitiveComponent.SetMaterial` _square_2 0 "/Game/Core/Cells/MI_Biome_Ocean.MI_Biome_Ocean")
        (`PrimitiveComponent.SetMaterial` (`self.Hexagon`) 0 "/Game/Core/Cells/MI_Biome_Ocean.MI_Biome_Ocean"))
      (:`NewEnumerator9`
        (`PrimitiveComponent.SetMaterial` _square_2 0 "/Game/Core/Cells/MI_Biome_Taiga.MI_Biome_Taiga")
        (`PrimitiveComponent.SetMaterial` (`self.Hexagon`) 0 "/Game/Core/Cells/MI_Biome_Taiga.MI_Biome_Taiga"))
      (:`NewEnumerator8`
        (`PrimitiveComponent.SetMaterial` _square_2 0 "/Game/Core/Cells/MI_Biome_TempForest.MI_Biome_TempForest")
        (`PrimitiveComponent.SetMaterial` (`self.Hexagon`) 0 "/Game/Core/Cells/MI_Biome_TempForest.MI_Biome_TempForest"))
      (:`NewEnumerator7`
        (`PrimitiveComponent.SetMaterial` _square_2 0 "/Game/Core/Cells/MI_Biome_TropicalForest.MI_Biome_TropicalForest")
        (`PrimitiveComponent.SetMaterial` (`self.Hexagon`) 0 "/Game/Core/Cells/MI_Biome_TropicalForest.MI_Biome_TropicalForest"))
      (:`NewEnumerator10`
        (`PrimitiveComponent.SetMaterial` _square_2 0 "/Game/Core/Cells/MI_Biome_Tundra.MI_Biome_Tundra")
        (`PrimitiveComponent.SetMaterial` (`self.Hexagon`) 0 "/Game/Core/Cells/MI_Biome_Tundra.MI_Biome_Tundra"))
      (:`NewEnumerator11`
        (`PrimitiveComponent.SetMaterial` _square_2 0 "/Game/Core/Cells/MI_Biome_Volcanic.MI_Biome_Volcanic")
        (`PrimitiveComponent.SetMaterial` (`self.Hexagon`) 0 "/Game/Core/Cells/MI_Biome_Volcanic.MI_Biome_Volcanic")))
    (else
      (bind _output_get (set `self.Biome` Biome))
      (switch `/Game/Core/Cells/Biome_Enum` _output_get
        (:`NewEnumerator0`
          (`PrimitiveComponent.SetMaterial` _square 0 "/Game/Core/Cells/MI_Biome_Desert.MI_Biome_Desert")
          (`PrimitiveComponent.SetMaterial` (`self.Hexagon`) 0 "/Game/Core/Cells/MI_Biome_Desert.MI_Biome_Desert"))
        (:`NewEnumerator1`
          (`PrimitiveComponent.SetMaterial` _square 0 "/Game/Core/Cells/MI_Biome_Grasslands.MI_Biome_Grasslands")
          (`PrimitiveComponent.SetMaterial` (`self.Hexagon`) 0 "/Game/Core/Cells/MI_Biome_Grasslands.MI_Biome_Grasslands"))
        (:`NewEnumerator12`
          (`PrimitiveComponent.SetMaterial` _square 0 "/Game/Core/Cells/MI_Biome_Marsh.MI_Biome_Marsh")
          (`PrimitiveComponent.SetMaterial` (`self.Hexagon`) 0 "/Game/Core/Cells/MI_Biome_Marsh.MI_Biome_Marsh"))
        (:`NewEnumerator3`
          (`PrimitiveComponent.SetMaterial` _square 0 "/Game/Core/Cells/MI_Biome_Ocean.MI_Biome_Ocean")
          (`PrimitiveComponent.SetMaterial` (`self.Hexagon`) 0 "/Game/Core/Cells/MI_Biome_Ocean.MI_Biome_Ocean"))
        (:`NewEnumerator9`
          (`PrimitiveComponent.SetMaterial` _square 0 "/Game/Core/Cells/MI_Biome_Taiga.MI_Biome_Taiga")
          (`PrimitiveComponent.SetMaterial` (`self.Hexagon`) 0 "/Game/Core/Cells/MI_Biome_Taiga.MI_Biome_Taiga"))
        (:`NewEnumerator8`
          (`PrimitiveComponent.SetMaterial` _square 0 "/Game/Core/Cells/MI_Biome_TempForest.MI_Biome_TempForest")
          (`PrimitiveComponent.SetMaterial` (`self.Hexagon`) 0 "/Game/Core/Cells/MI_Biome_TempForest.MI_Biome_TempForest"))
        (:`NewEnumerator7`
          (`PrimitiveComponent.SetMaterial` _square 0 "/Game/Core/Cells/MI_Biome_TropicalForest.MI_Biome_TropicalForest")
          (`PrimitiveComponent.SetMaterial` (`self.Hexagon`) 0 "/Game/Core/Cells/MI_Biome_TropicalForest.MI_Biome_TropicalForest"))
        (:`NewEnumerator10`
          (`PrimitiveComponent.SetMaterial` _square 0 "/Game/Core/Cells/MI_Biome_Tundra.MI_Biome_Tundra")
          (`PrimitiveComponent.SetMaterial` (`self.Hexagon`) 0 "/Game/Core/Cells/MI_Biome_Tundra.MI_Biome_Tundra"))
        (:`NewEnumerator11`
          (`PrimitiveComponent.SetMaterial` _square 0 "/Game/Core/Cells/MI_Biome_Volcanic.MI_Biome_Volcanic")
          (`PrimitiveComponent.SetMaterial` (`self.Hexagon`) 0 "/Game/Core/Cells/MI_Biome_Volcanic.MI_Biome_Volcanic"))))))

(fn `setCoordinates`
  (params (Coordinates :type "/Game/Core/HexCoordinates Structure") (Index :type Integer))
  ;[1 1 1] Set Coordinates and Index
  (set `self.HexCoordinates` (make `/Game/Core/RegCoordinates` Coordinates_X_5_9E55E313431F7B89311DF296FC8C0563 Coordinates_Z_7_4FE6599F458540090D6B3EB2C4F49AB6))
  (set `self.GridIndex` Index)
  ;[1 1 1] Display Coordinates and Index on Tile
  (`TextRenderComponent.K2_SetText` (`self.CoordinatesText`) (`KismetTextLibrary.Conv_StringToText` (`KismetStringLibrary.Concat_StrStr` (`KismetStringLibrary.Conv_IntToString` Coordinates_X_5_9E55E313431F7B89311DF296FC8C0563) "," (`KismetStringLibrary.Conv_IntToString` (`self.getHexYCoord` Coordinates_X_5_9E55E313431F7B89311DF296FC8C0563 Coordinates_Z_7_4FE6599F458540090D6B3EB2C4F49AB6)) "," (`KismetStringLibrary.Conv_IntToString` Coordinates_Z_7_4FE6599F458540090D6B3EB2C4F49AB6) "<br>" (`KismetStringLibrary.Conv_IntToString` Index)))))

(fn `setNeighbor`
  (params (Direction :type "/Game/Core/Cells/HexDirection_Enum Enum" :default "NewEnumerator0") (Cell :type "/Game/Core/Cells/BP_Cell Object Reference"))
  (`KismetArrayLibrary.Array_Set` (`self.Neighbors`) (`KismetMathLibrary.Conv_ByteToInt` Direction) Cell)
  (`KismetArrayLibrary.Array_Set` (`/Game/Core/Cells/BP_Cell.Neighbors` Cell) (`KismetMathLibrary.Conv_ByteToInt` (`self.getOppositeDirection` Direction)) self))

(fn `setShape`
  (params (`Hexagon?` :type Boolean))
  (if `Hexagon?`
    (`SceneComponent.SetVisibility` (`self.Hexagon`) true false)
    (`SceneComponent.SetVisibility` (`self.Square`) false false)
    (else
      (`SceneComponent.SetVisibility` (`self.Hexagon`) false false)
      (`SceneComponent.SetVisibility` (`self.Square`) true false)))
  (return))

(fn `UserConstructionScript`
  (`self.setShape` (`self.Hex?`))
  (`self.setBiome` true "NewEnumerator3"))