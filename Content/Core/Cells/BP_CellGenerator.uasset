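; BP_CellGenerator builds the game's grid of BP_Cell actors at BeginPlay, in either a hex or square layout.
; The construction script sizes the Tiles array from GridSize, then nested loops spawn each cell, set its shape and coordinates, and store it by running index.
; A FlipFlop staggers alternate hex rows by half a cell.
; GetCell and GetRandomCell read the flat array; RaiseTerrain is an empty stub.
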(event `self.ReceiveBeginPlay`
  (bind (_gridsize_x _gridsize_z) (break `/Game/Core/RegCoordinates` (`self.GridSize`)))
  (bind _tiles (`self.Tiles`))
  (bind _currentindex (`self.CurrentIndex`))
  (bind (_gridsize_x_2 _gridsize_z_2) (break `/Game/Core/RegCoordinates` (`self.GridSize`)))
  (bind _currentindex_2 (`self.CurrentIndex`))
  (bind _currentindex_3 (`self.CurrentIndex`))
  (bind _hex_ (`self.Hex?`))
  (bind _returnvalue (- _gridsize_z_2 1))
  (if (`self.Hex?`)
    ;[0.4769 1 0.6925] Create Hex Grid
    (for _index (range _gridsize_x_2)
      (`/Engine/EditorBlueprintResources/StandardMacros.FlipFlop`
        (:`A`
          (for _index_2 (range (+ _returnvalue 1))
            (bind _returnvalue_2 (* _index 75.0))
            (bind _returnvalue_3 (`|SpawnActorFromClass` "/Game/Core/Cells/BP_Cell.BP_Cell_C" (`KismetMathLibrary.MakeTransform` (`KismetMathLibrary.MakeVector` _returnvalue_2 (* _index_2 86.5))) "Undefined" "OverrideRootScale" null null))
            (`/Game/Core/Cells/BP_Cell.SetShape` _returnvalue_3 _hex_)
            (`/Game/Core/Cells/BP_Cell.FromOffsetCoordinates` _returnvalue_3 (make `/Game/Core/RegCoordinates` _index_2 _index))
            (bind _hexcoordinates (`/Game/Core/Cells/BP_Cell.FromOffsetCoordinates` _returnvalue_3 (make `/Game/Core/RegCoordinates` _index_2 _index)))
            (`/Game/Core/Cells/BP_Cell.SetCoordinates` _returnvalue_3 _hexcoordinates _currentindex)
            (`KismetArrayLibrary.Array_Set` _tiles _currentindex_2 _returnvalue_3)
            (`/Engine/EditorBlueprintResources/StandardMacros.IncrementInt` (`self.CurrentIndex`) :!label _label)))
        (:`B`
          (for _index_3 (range (+ _returnvalue 1))
            (bind _returnvalue_4 (`|SpawnActorFromClass` "/Game/Core/Cells/BP_Cell.BP_Cell_C" (`KismetMathLibrary.MakeTransform` (`KismetMathLibrary.MakeVector` _returnvalue_2 (+ (* _index_3 86.5) 43.25))) "Undefined" "OverrideRootScale" null null))
            (`/Game/Core/Cells/BP_Cell.SetShape` _returnvalue_4 _hex_)
            (bind _hexcoordinates_2 (`/Game/Core/Cells/BP_Cell.FromOffsetCoordinates` _returnvalue_4 (make `/Game/Core/RegCoordinates` _index_3 _index)))
            (`/Game/Core/Cells/BP_Cell.SetCoordinates` _returnvalue_4 _hexcoordinates_2 _currentindex)
            (`KismetArrayLibrary.Array_Set` _tiles _currentindex_2 _returnvalue_4)
            (goto _label)))))
    (else
      ;[1 0.7952 0.6084] Create Square Grid
      (for _index_4 (range _gridsize_x)
        (for _index_5 (range _gridsize_z)
          (bind _returnvalue_5 (`|SpawnActorFromClass` "/Game/Core/Cells/BP_Cell.BP_Cell_C" (`KismetMathLibrary.MakeTransform` (`KismetMathLibrary.MakeVector` (* _index_5 100.0) (* _index_4 100.0))) "Undefined" "OverrideRootScale" null null))
          (`/Game/Core/Cells/BP_Cell.SetShape` _returnvalue_5 (`self.Hex?`))
          (bind _hexcoordinates_3 (`/Game/Core/Cells/BP_Cell.FromOffsetCoordinates` _returnvalue_5 (make `/Game/Core/RegCoordinates` _index_5 _index_4)))
          (`/Game/Core/Cells/BP_Cell.SetCoordinates` _returnvalue_5 _hexcoordinates_3 _currentindex_3)
          (`KismetArrayLibrary.Array_Set` (`self.Tiles`) _currentindex_3 _returnvalue_5)
          (`/Engine/EditorBlueprintResources/StandardMacros.IncrementInt` (`self.CurrentIndex`)))))))

(fn `GetCell`
  (params (Coordinate :type "/Game/Core/RegCoordinates Structure"))
  (returns (CellRef :type "/Game/Core/Cells/BP_Cell Object Reference"))
  (bind _gridsize_x (break `/Game/Core/RegCoordinates` (`self.GridSize`)))
  (return (`|GetArrayItem` (`self.Tiles`) (+ Coordinate_X_5_0D60888443DB7109C5060C8AE787FDE6 (* Coordinate_Z_7_1B0FBEA646C06A4A8B3183871708624D _gridsize_x)))))

(fn `GetRandomCell`
  (returns (Cell :type "/Game/Core/Cells/BP_Cell Object Reference"))
  (bind (_gridsize_x _gridsize_z) (break `/Game/Core/RegCoordinates` (`self.GridSize`)))
  (bind _cellref (`self.GetCell` (make `/Game/Core/RegCoordinates` (`KismetMathLibrary.RandomIntegerInRange` 0 (- _gridsize_x 1)) (`KismetMathLibrary.RandomIntegerInRange` 0 (- _gridsize_z 1)))))
  (return _cellref))

(fn `RaiseTerrain`
  (params (chunkSize :type Integer)))

(fn `UserConstructionScript`
  (bind (_gridsize_x _gridsize_z) (break `/Game/Core/RegCoordinates` (`self.GridSize`)))
  (bind _returnvalue (* _gridsize_x _gridsize_z))
  (`KismetArrayLibrary.Array_Resize` (`self.Tiles`) _returnvalue)
  (set `self.CellCount` _returnvalue))