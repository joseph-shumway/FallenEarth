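; Player actor for a hex map: shows the mouse cursor, controls the camera and forwards click input to the grid.
; Holding right-click drags the camera and scrolling zooms along its forward vector, both scaled by height.
; Held left-click calls the grid's LClick every fourth tick through nested FlipFlops and a Gate; Shift+left-click calls ShiftLClick.
; Spacebar tells the HexMapGenerator found at BeginPlay to recreate the map.
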(event `self.ReceiveBeginPlay`
  (bind _returnvalue (`GameplayStatics.GetPlayerController` 0))
  ;[1 1 1] Activate Mouse Cursor and get a reference to the Hex Generator to stor in GridRef
  (`PlayerController.SetViewTargetWithBlend` _returnvalue self 1.0 "VTBlend_Linear" 0.0 false)
  (set `PlayerController.bShowMouseCursor` true _returnvalue)
  (bind _outactors (`GameplayStatics.GetAllActorsOfClass` "/Game/Core/Cells/HexMapGenerator.HexMapGenerator_C"))
  (bind _output (`|GetArrayItem` _outactors))
  (set `self.GeneratorRef` _output)
  (set `self.GridRef` (`/Game/Core/Cells/HexMapGenerator.HexGridRef` _output)))

(event `InputAxis|MouseHoriz`
  (params (AxisValue :type "Float (single-precision)"))
  (bind (_returnvalue_x _returnvalue_y _returnvalue_z) (`KismetMathLibrary.BreakVector` (`self.K2_GetActorLocation`)))
  (bind _returnvalue (/ _returnvalue_z 275.0))
  ;[1 1 1] Camera Movement
  (`/Engine/EditorBlueprintResources/StandardMacros.Gate` true :!label _label
    (:`Exit`
      (`self.K2_AddActorWorldOffset` (`KismetMathLibrary.MakeVector` 0.0 (* _returnvalue (* -11 AxisValue))))
      (`self.K2_AddActorWorldOffset` (`KismetMathLibrary.MakeVector` (* _returnvalue (* -11 (`self.GetInputAxisValue`))))))))

(event `InputAction|RClick`
  (params (Key :type "Key Structure"))
  ;[1 1 1] Camera Movement
  (:`Pressed`
    (goto _label :!via `Open`))
  (:`Released`
    (goto _label :!via `Close`)))

(event `self.ReceiveTick`
  (params (DeltaSeconds :type "Float (single-precision)"))
  (`/Engine/EditorBlueprintResources/StandardMacros.FlipFlop`
    (:`A`
      (`/Engine/EditorBlueprintResources/StandardMacros.FlipFlop`
        (:`A`
          ;[1 1 1] Input to send to grid
          (`/Engine/EditorBlueprintResources/StandardMacros.Gate` true :!label _label_2
            (:`Exit`
              (`/Game/Core/Cells/HexGrid.LClick` (`self.GridRef`)))))))))

(event `InputAction|LClick`
  (params (Key :type "Key Structure"))
  ;[1 1 1] Input to send to grid
  (:`Pressed`
    (goto _label_2 :!via `Open`))
  (:`Released`
    (goto _label_2 :!via `Close`)))

(event `InputAction|ShiftLClick`
  (params (Key :type "Key Structure"))
  ;[1 1 1] Input to send to grid
  (:`Pressed`
    (`/Game/Core/Cells/HexGrid.ShiftLClick` (`self.GridRef`))))

(event `Key|SpaceBar`
  (params (Key :type "Key Structure"))
  (:`Pressed`
    (`/Game/Core/Cells/HexMapGenerator.RecreateMap` (`self.GeneratorRef`))))

(event `InputAxis|ScrollDown`
  (params (AxisValue :type "Float (single-precision)"))
  (bind (_returnvalue_x _returnvalue_y _returnvalue_z) (`KismetMathLibrary.BreakVector` (`self.K2_GetActorLocation`)))
  (`self.K2_AddActorWorldOffset` (* (`SceneComponent.GetForwardVector` (`self.Camera`)) (* (* AxisValue (`self.ZoomSensitivity`)) (/ _returnvalue_z 100.0)))))

(fn `UserConstructionScript`)