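; BP_TileGenerator is an actor that spawns a flat grid of BP_Tile actors when play begins.
; The construction script sizes the Tiles array to the product of the two GridSize dimensions.
; BeginPlay runs nested loops over those dimensions, placing tiles at fixed spacing along X and Y and writing each into Tiles by an incremented index.
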(event `self.ReceiveBeginPlay`
  (bind (_gridsize_value1 _gridsize_value2) (break `/Game/Core/Int2D` (`self.GridSize`)))
  (for _index (range _gridsize_value1)
    (for _index_2 (range _gridsize_value2)
      (bind _returnvalue (`|SpawnActorFromClass` "/Game/Core/BP_Tile.BP_Tile_C" (`KismetMathLibrary.MakeTransform` (`KismetMathLibrary.MakeVector` (* _index 100.0) (* _index_2 100.0))) "Undefined" "OverrideRootScale" null null))
      (`KismetArrayLibrary.Array_Set` (`self.Tiles`) (`self.Index`) _returnvalue)
      (`/Engine/EditorBlueprintResources/StandardMacros.IncrementInt` (`self.Index`)))))

(fn `UserConstructionScript`
  (bind (_gridsize_value1 _gridsize_value2) (break `/Game/Core/Int2D` (`self.GridSize`)))
  (`KismetArrayLibrary.Array_Resize` (`self.Tiles`) (* _gridsize_value1 _gridsize_value2)))